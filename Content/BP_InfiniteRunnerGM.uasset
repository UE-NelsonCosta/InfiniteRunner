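; Game mode Blueprint for an infinite runner that can report whether any spawned character is still alive.
; On BeginPlay it finds and caches the BP_CharacterSpawnerManager in the level.
; IsThereACharacterAlive loops over the manager's spawned characters, casts each to FemaleCharacter or MaleCharacter, and returns true at the first one alive.
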(event `self.ReceiveBeginPlay`
  (bind _returnvalue (`GameplayStatics.GetActorOfClass` "/Game/Blueprints/BP_CharacterSpawnerManager.BP_CharacterSpawnerManager_C"))
  (set `self.CharacterSpawnerManager` _returnvalue))

(fn `IsThereACharacterAlive`
  (returns (ReturnValue :type Boolean))
  (for _array_element (`CharacterSpawnerManager.SpawnedCharacters` (`self.CharacterSpawnerManager`))
    (bind _asfemale_character (cast `/Game/Blueprints/FemaleCharacter` _array_element)
      (:`then`
        (if (`/Game/Blueprints/FemaleCharacter.IsAlive` _asfemale_character)
          (return true)))
      (:`CastFailed`
        (bind _asmale_character (cast `/Game/Blueprints/MaleCharacter` _array_element))
        (if (`/Game/Blueprints/MaleCharacter.IsAlive` _asmale_character)
          (return true)))))
  (return false))

(fn `UserConstructionScript`)