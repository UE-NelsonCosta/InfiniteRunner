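; BP_CharacterSpawner is an actor that spawns a set of characters at player start points when play begins.
; BeginPlay loops over PlayerStarts, spawns the CharactersToSpawn class at the same index with that start's transform, ignoring collisions, and records each in SpawnedCharacters.
; GetMiddleMostCharacter returns the entry at half the length of SpawnedCharacters, so the middle is decided by array order rather than position.
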(event `self.ReceiveBeginPlay`
  (bind _result (`/Engine/EditorBlueprintResources/StandardMacros.DecrementInt` (`KismetArrayLibrary.Array_Length` (`self.PlayerStarts`)))
    (:`  `
      (for _index (range (+ _result 1))
        (bind _returnvalue (`|SpawnActorFromClass` (`|GetArrayItem` (`self.CharactersToSpawn`) _index) (`self.GetTransform` (`|GetArrayItem` (`self.PlayerStarts`) _index)) "AlwaysSpawn" "OverrideRootScale" null null))
        (`KismetArrayLibrary.Array_AddUnique` (`self.SpawnedCharacters`) _returnvalue)))))

(fn `GetMiddleMostCharacter`
  (returns (Character :type "Character Object Reference"))
  (return (`|GetArrayItem` (`self.SpawnedCharacters`) (/ (`KismetArrayLibrary.Array_Length` (`self.SpawnedCharacters`)) 2))))

(fn `UserConstructionScript`)